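; Tower of Hanoi minigame (phase 4): arrow keys cycle a pointer over three columns, Space picks up or drops a piece.
; Column arrays act as stacks of ID/piece structs, seeded with five pieces in Iniciar2; drops reject larger IDs on smaller ones and snap to preset Posicoes slots.
; Moves and errors are counted; filling column 3 records both plus elapsed time in GI_Jogo and shows FimFase4.
; Inicializar creates the countdown widget.
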(event EventBeginPlay)

(event Input|KeyboardEvents|Left
  (params (Key :type Key%20Structure))
  (:Pressed
    (bind _output_get (Variables|Default|SetPosicaoSeta (+ (Variables|Default|GetPosicaoSeta) -1)))
    (if (== _output_get 0)
      (Variables|Default|SetPosicaoSeta 3))
    (CallFunction|MoverSeta)))

(event Input|KeyboardEvents|SpaceBar
  (params (Key :type Key%20Structure))
  (:Pressed
    (if (Variables|Default|GetEstaSegurandoPeca)
      (CallFunction|Soltarpeça)
      (else
        (CallFunction|Pegarpeca)))))

(event Input|KeyboardEvents|Right
  (params (Key :type Key%20Structure))
  (:Pressed
    (bind _output_get (Variables|Default|SetPosicaoSeta (+ (Variables|Default|GetPosicaoSeta) 1)))
    (if (== _output_get 4)
      (Variables|Default|SetPosicaoSeta 1))
    (CallFunction|MoverSeta)))

(fn ConstructionScript)

(fn MoverSeta
  (bind _seta (Variables|Default|GetSeta))
  (switch int (Variables|Default|GetPosicaoSeta)
    (:1
      (Transformation|SetRelativeLocation _seta "0.000000,650.000000,760.000000" true false))
    (:2
      (Transformation|SetRelativeLocation _seta "0.000000,0.000000,760.000000" true false))
    (:3
      (Transformation|SetRelativeLocation _seta "0.000000,-650.000000,760.000000" true false)))
  (if (Variables|Default|GetEstaSegurandoPeca)
    (switch int (Variables|Default|GetPosicaoSeta)
      (:1
        _)
      (:2
        _)
      (:3
        _))
    (CallFunction|Subirpeca (.Peca (Utilities|Struct|BreakES_Peca (Variables|Default|GetPecaSegurada))))))

(fn Soltarpeça
  (bind _coluna2 (Variables|Default|GetColuna2))
  (bind _coluna2_2 (Variables|Default|GetColuna2))
  (bind _coluna3 (Variables|Default|GetColuna3))
  (bind _coluna3_2 (Variables|Default|GetColuna3))
  (bind _pecasegurada (Variables|Default|GetPecaSegurada))
  (bind _pecasegurada_2 (Variables|Default|GetPecaSegurada))
  (bind _pecasegurada_3 (Variables|Default|GetPecaSegurada))
  (bind _pecasegurada_4 (Variables|Default|GetPecaSegurada))
  (bind _pecasegurada_5 (Variables|Default|GetPecaSegurada))
  (bind _pecasegurada_6 (Variables|Default|GetPecaSegurada))
  (bind _coluna1 (Variables|Default|GetColuna1))
  (bind _pecasegurada_7 (Variables|Default|GetPecaSegurada))
  (bind _pecasegurada_8 (Variables|Default|GetPecaSegurada))
  (bind _pecasegurada_9 (Variables|Default|GetPecaSegurada))
  (bind _pecasegurada_10 (Variables|Default|GetPecaSegurada))
  (bind _pecasegurada_11 (Variables|Default|GetPecaSegurada))
  (bind _pecasegurada_12 (Variables|Default|GetPecaSegurada))
  (bind _coluna1_2 (Variables|Default|GetColuna1))
  (bind _pecasegurada_13 (Variables|Default|GetPecaSegurada))
  (bind _pecasegurada_14 (Variables|Default|GetPecaSegurada))
  (bind _pecasegurada_15 (Variables|Default|GetPecaSegurada))
  (bind _returnvalue (Utilities|Array|Length _coluna3))
  (bind _returnvalue_2 (Utilities|Array|Length _coluna1_2))
  (bind _returnvalue_3 (Utilities|Array|Length _coluna2_2))
  (switch int (Variables|Default|GetPosicaoSeta)
    (:1
      (if (Utilities|Array|IsEmpty _coluna1)
        (Transformation|SetRelativeLocation (.Peca (Utilities|Struct|BreakES_Peca _pecasegurada_2)) (.Location (Math|Transform|BreakTransform (Utilities|Array|Get(acopy) (Variables|Default|GetPosicoes) 5))) true false :!label _label)
        (Utilities|Array|Add (Variables|Default|GetColuna1) _pecasegurada_2)
        (Variables|Default|SetEstaSegurandoPeca false :!label _label_2)
        (Audio|PlaySound2D "/Game/Assets/Sons/Clicke.Clicke" 1.0 1.0 0.0 0 0)
        (Variables|Default|SetTentativas (+ 1 (Variables|Default|GetTentativas)))
        (if (== (Utilities|Array|Length (Variables|Default|GetColuna3)) 5)
          (Audio|PlaySound2D "/Game/Assets/Sons/game-start-6104.game-start-6104" 1.0 1.0 0.0 0 0)
          (bind _asgi_jogo (Utilities|Casting|CastToGI_Jogo (Game|GetGameInstance)))
          (Default|RegistrarFase4 _asgi_jogo (Variables|Default|GetTentativas) (Math|Float|Truncate (- (Utilities|Time|GetGameTimeinSeconds) (Variables|Default|GetTempo%20inicial))) (Variables|Default|GetTentativasErradas))
          (bind _returnvalue_4 (UserInterface|CreateWidget "/Game/Widgets/FimFase4.FimFase4_C"))
          (UserInterface|Viewport|AddtoViewport _returnvalue_4 0))
        (elif (> (.ID (Utilities|Struct|BreakES_Peca (Variables|Default|GetPecaSegurada))) (.ID (Utilities|Struct|BreakES_Peca (Utilities|Array|Get(acopy) _coluna1 (Utilities|Array|LastIndex _coluna1)))))
          (if (== _returnvalue_2 0)
            (switch int _returnvalue_2 :!label _label_3
              (:0
                (goto _label))
              (:1
                (Transformation|SetRelativeLocation (.Peca (Utilities|Struct|BreakES_Peca _pecasegurada_13)) (.Location (Math|Transform|BreakTransform (Utilities|Array|Get(acopy) (Variables|Default|GetPosicoes) 4))) true false)
                (Utilities|Array|Add (Variables|Default|GetColuna1) _pecasegurada_13)
                (goto _label_2))
              (:2
                (Transformation|SetRelativeLocation (.Peca (Utilities|Struct|BreakES_Peca _pecasegurada_15)) (.Location (Math|Transform|BreakTransform (Utilities|Array|Get(acopy) (Variables|Default|GetPosicoes) 3))) true false)
                (Utilities|Array|Add (Variables|Default|GetColuna1) _pecasegurada_15)
                (goto _label_2))
              (:3
                (Transformation|SetRelativeLocation (.Peca (Utilities|Struct|BreakES_Peca _pecasegurada_14)) (.Location (Math|Transform|BreakTransform (Utilities|Array|Get(acopy) (Variables|Default|GetPosicoes) 2))) true false)
                (Utilities|Array|Add (Variables|Default|GetColuna1) _pecasegurada_14)
                (goto _label_2))
              (:4
                (Transformation|SetRelativeLocation (.Peca (Utilities|Struct|BreakES_Peca _pecasegurada_12)) (.Location (Math|Transform|BreakTransform (Utilities|Array|Get(acopy) (Variables|Default|GetPosicoes) 1))) true false)
                (Utilities|Array|Add (Variables|Default|GetColuna1) _pecasegurada_12)
                (goto _label_2)))
            (else
              (Audio|PlaySound2D "/Game/Assets/Sons/Wrong.Wrong" 1.0 1.0 0.0 0 0)
              (Variables|Default|SetTentativasErradas (+ 1 (Variables|Default|GetTentativasErradas)))))
          (else
            (goto _label_3)))))
    (:2
      (if (Utilities|Array|IsEmpty _coluna2)
        (Transformation|SetRelativeLocation (.Peca (Utilities|Struct|BreakES_Peca _pecasegurada_11)) (.Location (Math|Transform|BreakTransform (Utilities|Array|Get(acopy) (Variables|Default|GetPosicoes) 10))) true false :!label _label_4)
        (Utilities|Array|Add (Variables|Default|GetColuna2) _pecasegurada_11)
        (goto _label_2)
        (elif (> (.ID (Utilities|Struct|BreakES_Peca (Variables|Default|GetPecaSegurada))) (.ID (Utilities|Struct|BreakES_Peca (Utilities|Array|Get(acopy) _coluna2 (Utilities|Array|LastIndex _coluna2)))))
          (if (== _returnvalue_3 0)
            (switch int _returnvalue_3 :!label _label_5
              (:0
                (goto _label_4))
              (:1
                (Transformation|SetRelativeLocation (.Peca (Utilities|Struct|BreakES_Peca _pecasegurada_10)) (.Location (Math|Transform|BreakTransform (Utilities|Array|Get(acopy) (Variables|Default|GetPosicoes) 9))) true false)
                (Utilities|Array|Add (Variables|Default|GetColuna2) _pecasegurada_10)
                (goto _label_2))
              (:2
                (Transformation|SetRelativeLocation (.Peca (Utilities|Struct|BreakES_Peca _pecasegurada_9)) (.Location (Math|Transform|BreakTransform (Utilities|Array|Get(acopy) (Variables|Default|GetPosicoes) 8))) true false)
                (Utilities|Array|Add (Variables|Default|GetColuna2) _pecasegurada_9)
                (goto _label_2))
              (:3
                (Transformation|SetRelativeLocation (.Peca (Utilities|Struct|BreakES_Peca _pecasegurada_8)) (.Location (Math|Transform|BreakTransform (Utilities|Array|Get(acopy) (Variables|Default|GetPosicoes) 7))) true false)
                (Utilities|Array|Add (Variables|Default|GetColuna2) _pecasegurada_8)
                (goto _label_2))
              (:4
                (Transformation|SetRelativeLocation (.Peca (Utilities|Struct|BreakES_Peca _pecasegurada_7)) (.Location (Math|Transform|BreakTransform (Utilities|Array|Get(acopy) (Variables|Default|GetPosicoes) 6))) true false)
                (Utilities|Array|Add (Variables|Default|GetColuna2) _pecasegurada_7)
                (goto _label_2)))
            (else
              (Audio|PlaySound2D "/Game/Assets/Sons/Wrong.Wrong" 1.0 1.0 0.0 0 0)
              (Variables|Default|SetTentativasErradas (+ 1 (Variables|Default|GetTentativasErradas)))))
          (else
            (goto _label_5)))))
    (:3
      (if (Utilities|Array|IsEmpty _coluna3_2)
        (Transformation|SetRelativeLocation (.Peca (Utilities|Struct|BreakES_Peca _pecasegurada_6)) (.Location (Math|Transform|BreakTransform (Utilities|Array|Get(acopy) (Variables|Default|GetPosicoes) 15))) true false :!label _label_6)
        (Utilities|Array|Add (Variables|Default|GetColuna3) _pecasegurada_6)
        (goto _label_2)
        (elif (> (.ID (Utilities|Struct|BreakES_Peca (Variables|Default|GetPecaSegurada))) (.ID (Utilities|Struct|BreakES_Peca (Utilities|Array|Get(acopy) _coluna3_2 (Utilities|Array|LastIndex _coluna3_2)))))
          (if (== _returnvalue 0)
            (switch int _returnvalue :!label _label_7
              (:0
                (goto _label_6))
              (:1
                (Transformation|SetRelativeLocation (.Peca (Utilities|Struct|BreakES_Peca _pecasegurada_3)) (.Location (Math|Transform|BreakTransform (Utilities|Array|Get(acopy) (Variables|Default|GetPosicoes) 14))) true false)
                (Utilities|Array|Add (Variables|Default|GetColuna3) _pecasegurada_3)
                (goto _label_2))
              (:2
                (Transformation|SetRelativeLocation (.Peca (Utilities|Struct|BreakES_Peca _pecasegurada_4)) (.Location (Math|Transform|BreakTransform (Utilities|Array|Get(acopy) (Variables|Default|GetPosicoes) 13))) true false)
                (Utilities|Array|Add (Variables|Default|GetColuna3) _pecasegurada_4)
                (goto _label_2))
              (:3
                (Transformation|SetRelativeLocation (.Peca (Utilities|Struct|BreakES_Peca _pecasegurada_5)) (.Location (Math|Transform|BreakTransform (Utilities|Array|Get(acopy) (Variables|Default|GetPosicoes) 12))) true false)
                (Utilities|Array|Add (Variables|Default|GetColuna3) _pecasegurada_5)
                (goto _label_2))
              (:4
                (Transformation|SetRelativeLocation (.Peca (Utilities|Struct|BreakES_Peca _pecasegurada)) (.Location (Math|Transform|BreakTransform (Utilities|Array|Get(acopy) (Variables|Default|GetPosicoes) 11))) true false)
                (Utilities|Array|Add (Variables|Default|GetColuna3) _pecasegurada)
                (goto _label_2)))
            (else
              (Audio|PlaySound2D "/Game/Assets/Sons/Wrong.Wrong" 1.0 1.0 0.0 0 0)
              (Variables|Default|SetTentativasErradas (+ 1 (Variables|Default|GetTentativasErradas)))))
          (else
            (goto _label_7)))))))

(fn Pegarpeca
  (bind _coluna2 (Variables|Default|GetColuna2))
  (bind _coluna3 (Variables|Default|GetColuna3))
  (bind _coluna1 (Variables|Default|GetColuna1))
  (bind _coluna1_2 (Variables|Default|GetColuna1))
  (bind _returnvalue (Utilities|Array|LastIndex _coluna2))
  (bind _returnvalue_2 (Utilities|Array|LastIndex _coluna1_2))
  (bind _returnvalue_3 (Utilities|Array|LastIndex _coluna3))
  (bind _output (Utilities|Array|Get(acopy) _coluna2 _returnvalue))
  (bind _output_2 (Utilities|Array|Get(acopy) _coluna1_2 _returnvalue_2))
  (bind _output_3 (Utilities|Array|Get(acopy) _coluna3 _returnvalue_3))
  (bind (_id _peca) (Utilities|Struct|BreakES_Peca _output))
  (bind (_id_2 _peca_2) (Utilities|Struct|BreakES_Peca _output_3))
  (bind (_id_3 _peca_3) (Utilities|Struct|BreakES_Peca _output_2))
  (switch int (Variables|Default|GetPosicaoSeta)
    (:1
      (if (== (Utilities|Array|Length (Variables|Default|GetColuna1)) 0)
        (Audio|PlaySound2D "/Game/Assets/Sons/Wrong.Wrong" 1.0 1.0 0.0 0 0 :!label _label)
        (Variables|Default|SetTentativasErradas (+ (Variables|Default|GetTentativasErradas) 1))
        (else
          (CallFunction|Subirpeca _peca_3)
          (Variables|Default|SetPecaSegurada (Utilities|Struct|MakeES_Peca _id_3 _peca_3))
          (Utilities|Array|RemoveIndex _coluna1 (Utilities|Array|LastIndex _coluna1))
          (Variables|Default|SetEstaSegurandoPeca true :!label _label_2))))
    (:2
      (if (== (Utilities|Array|Length (Variables|Default|GetColuna2)) 0)
        (goto _label)
        (else
          (CallFunction|Subirpeca _peca)
          (Variables|Default|SetPecaSegurada (Utilities|Struct|MakeES_Peca _id _peca))
          (Utilities|Array|RemoveIndex _coluna2 _returnvalue)
          (goto _label_2))))
    (:3
      (if (== (Utilities|Array|Length (Variables|Default|GetColuna3)) 0)
        (goto _label)
        (else
          (CallFunction|Subirpeca _peca_2)
          (Variables|Default|SetPecaSegurada (Utilities|Struct|MakeES_Peca _id_2 _peca_2))
          (Utilities|Array|RemoveIndex _coluna3 _returnvalue_3)
          (goto _label_2))))))

(fn Subirpeca
  (params (a%20mover :type Static%20Mesh%20Component%20Object%20Reference))
  (switch int (Variables|Default|GetPosicaoSeta)
    (:1
      (Transformation|SetRelativeLocation a%20mover "0.000000,650.000000,760.000000" false false))
    (:2
      (Transformation|SetRelativeLocation a%20mover "0.000000,0.000000,760.000000" false false))
    (:3
      (Transformation|SetRelativeLocation a%20mover "0.000000,-650.000000,760.000000" false false))))

(fn Inicializar
  (bind _returnvalue (UserInterface|CreateWidget "/Game/Widgets/WB_Contagem.WB_Contagem_C"))
  (Default|ComecarContagem _returnvalue)
  (UserInterface|SetWidget (Variables|Default|GetContagem) _returnvalue)
  (EventDispatchers|BindEventtoComecaAgora5 _returnvalue (EventDispatchers|CreateEvent :!event Iniciar2)))

(fn Iniciar2
  (bind _returnvalue (Actor|GetActorOfClass "/Script/Engine.AmbientSound"))
  (Audio|Components|Audio|SetSound (Variables|/Script/Engine.AmbientSound|GetAudioComponent _returnvalue) "/Game/Assets/Sons/Musicas/BemLeve.BemLeve")
  (Class|AudioComponent|SetPaused (Variables|/Script/Engine.AmbientSound|GetAudioComponent _returnvalue) false)
  (Variables|Default|SetPosicaoSeta 1)
  (Utilities|Array|Add (Variables|Default|GetColuna1) (Utilities|Struct|MakeES_Peca 5 (Variables|Default|Getpeca5)))
  (Utilities|Array|Add (Variables|Default|GetColuna1) (Utilities|Struct|MakeES_Peca 4 (Variables|Default|Getpeca4)))
  (Utilities|Array|Add (Variables|Default|GetColuna1) (Utilities|Struct|MakeES_Peca 3 (Variables|Default|Getpeca3)))
  (Utilities|Array|Add (Variables|Default|GetColuna1) (Utilities|Struct|MakeES_Peca 2 (Variables|Default|Getpeca2)))
  (Utilities|Array|Add (Variables|Default|GetColuna1) (Utilities|Struct|MakeES_Peca 1 (Variables|Default|Getpeca1))))
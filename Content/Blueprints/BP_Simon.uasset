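; BP_Simon runs the phase 2 Simon memory game, where players hit four coloured lights to repeat a random sequence.
; A looping timer plays the sequence with lights and sounds while hits are disabled.
; Each hit is checked immediately: completing the sequence extends it, while an error costs a life and restarts it.
; When lives run out, it records hits, time and longest sequence in GI_Jogo and shows the end screen.
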(event OnComponentHit(Amarelo4)
  (params (HitComponent :type Primitive%20Component%20Object%20Reference) (OtherActor :type Actor%20Object%20Reference) (OtherComp :type Primitive%20Component%20Object%20Reference) (NormalImpulse :type Vector :default "0, 0, 0") (Hit :type Hit%20Result%20Structure%20%28by%20ref%29))
  (bind _arraydojogador (Variables|Default|GetArrayDojogador))
  (bind _arraydojogador_2 (Variables|Default|GetArrayDojogador))
  (bind _referenciavidas (Variables|Default|GetReferenciaVidas))
  (bind _returnvalue (Utilities|Array|Length _arraydojogador))
  (bind _returnvalue_2 (Utilities|Array|LastIndex _arraydojogador_2))
  (if (not (Variables|Default|GetDesativarTiros))
    (Rendering|Material|SetMaterial (Variables|Default|GetAmarelo4) 0 "/Game/Materiais/Lazer_Amarelo.Lazer_Amarelo")
    (Audio|PlaySound2D "/Game/Assets/Sons/4.4" 1.0 1.0 0.0 0 0)
    (Utilities|Array|Add (Variables|Default|GetArrayDojogador) 1)
    (Utilities|FlowControl|Delay 0.2)
    (CallFunction|Apagar)
    (if (== (Utilities|Array|Get(acopy) (Variables|Default|GetArray) _returnvalue_2) (Utilities|Array|Get(acopy) (Variables|Default|GetArrayDojogador) _returnvalue_2))
      ;[1 1 1] Acertou/ é o ultimo acerto?
      (Variables|Default|SetAcertos (+ (Variables|Default|GetAcertos) 1))
      (if (== (Utilities|Array|LastIndex (Variables|Default|GetArrayDojogador)) (Utilities|Array|LastIndex (Variables|Default|GetArray)))
        ;[1 1 1] è a maior sequencia?
        (if (> _returnvalue (Variables|Default|GetMaiorSequencia))
          (Variables|Default|SetMaiorSequencia _returnvalue))
        (bind _outactors (Actor|GetAllActorsOfClass "/Game/Blueprints/BP_LuzCoringa.BP_LuzCoringa_C"))
        (for _array_element _outactors
          (Default|PiscarVerde _array_element))
        (Audio|PlaySound2D "/Game/Assets/Sons/CompletandoFase.CompletandoFase" 1.0 1.0 0.0 0 0)
        (Rendering|Material|SetMaterial (Variables|Default|GetVerde1) 0 "/Game/Materiais/Lazer_Verde.Lazer_Verde")
        (Rendering|Material|SetMaterial (Variables|Default|GetAmarelo4) 0 "/Game/Materiais/Lazer_Verde.Lazer_Verde")
        (Rendering|Material|SetMaterial (Variables|Default|GetVermelho3) 0 "/Game/Materiais/Lazer_Verde.Lazer_Verde")
        (Rendering|Material|SetMaterial (Variables|Default|GetAzul2) 0 "/Game/Materiais/Lazer_Verde.Lazer_Verde")
        (Utilities|Array|Clear (Variables|Default|GetArrayDojogador))
        (Utilities|FlowControl|Delay 0.5)
        (CallFunction|Apagar)
        (CallFunction|GerarSequencia)
        (CallFunction|IniciarSequencia)
        (else
          (Utilities|FlowControl|Delay 0.5)
          (CallFunction|Apagar)))
      (else
        ;[1 1 1] Erro
        (bind _outactors_2 (Actor|GetAllActorsOfClass "/Game/Blueprints/BP_LuzCoringa.BP_LuzCoringa_C"))
        (for _array_element_2 _outactors_2
          (Default|PiscarVermelho _array_element_2))
        (Audio|PlaySound2D "/Game/Assets/Sons/Wrong.Wrong" 1.0 1.0 0.0 0 0)
        (Rendering|Material|SetMaterial (Variables|Default|GetVerde1) 0 "/Game/Materiais/Lazer_Vermelho.Lazer_Vermelho")
        (Rendering|Material|SetMaterial (Variables|Default|GetAmarelo4) 0 "/Game/Materiais/Lazer_Vermelho.Lazer_Vermelho")
        (Rendering|Material|SetMaterial (Variables|Default|GetVermelho3) 0 "/Game/Materiais/Lazer_Vermelho.Lazer_Vermelho")
        (Rendering|Material|SetMaterial (Variables|Default|GetAzul2) 0 "/Game/Materiais/Lazer_Vermelho.Lazer_Vermelho")
        (Variables|Default|SetTentativasRestantes (- (Variables|Default|GetTentativasRestantes) 1))
        (Default|DiminuirContagem _referenciavidas)
        (UserInterface|SetWidget (Variables|Default|GetVidas) _referenciavidas)
        (if (== (Variables|Default|GetTentativasRestantes) 0)
          (bind _asgi_jogo (Utilities|Casting|CastToGI_Jogo (Game|GetGameInstance)))
          (Default|RegistrarFase2 _asgi_jogo (Variables|Default|GetAcertos) (Math|Float|Truncate (- (Utilities|Time|GetGameTimeinSeconds) (Variables|Default|GetTempoInicial))) (Variables|Default|GetMaiorSequencia))
          (bind _returnvalue_3 (UserInterface|CreateWidget "/Game/Widgets/FimFase2.FimFase2_C"))
          (UserInterface|Viewport|AddtoViewport _returnvalue_3 0)
          (else
            (Utilities|FlowControl|Delay 1.0)
            (CallFunction|Apagar)
            (Utilities|Array|Clear (Variables|Default|GetArrayDojogador))
            (Utilities|Array|Clear (Variables|Default|GetArray))
            (CallFunction|GerarSequencia)
            (CallFunction|IniciarSequencia)))))))

(event OnComponentHit(Verde1)
  (params (HitComponent :type Primitive%20Component%20Object%20Reference) (OtherActor :type Actor%20Object%20Reference) (OtherComp :type Primitive%20Component%20Object%20Reference) (NormalImpulse :type Vector :default "0, 0, 0") (Hit :type Hit%20Result%20Structure%20%28by%20ref%29))
  (bind _arraydojogador (Variables|Default|GetArrayDojogador))
  (bind _arraydojogador_2 (Variables|Default|GetArrayDojogador))
  (bind _referenciavidas (Variables|Default|GetReferenciaVidas))
  (bind _returnvalue (Utilities|Array|Length _arraydojogador))
  (bind _returnvalue_2 (Utilities|Array|LastIndex _arraydojogador_2))
  (if (not (Variables|Default|GetDesativarTiros))
    (Rendering|Material|SetMaterial (Variables|Default|GetVerde1) 0 "/Game/Materiais/Lazer_Verde.Lazer_Verde")
    (Audio|PlaySound2D "/Game/Assets/Sons/1.1" 1.0 1.0 0.0 0 0)
    (Utilities|Array|Add (Variables|Default|GetArrayDojogador) 0)
    (Utilities|FlowControl|Delay 0.2)
    (CallFunction|Apagar)
    (if (== (Utilities|Array|Get(acopy) (Variables|Default|GetArray) _returnvalue_2) (Utilities|Array|Get(acopy) (Variables|Default|GetArrayDojogador) _returnvalue_2))
      ;[1 1 1] Acertou/ é o ultimo acerto?
      (Variables|Default|SetAcertos (+ (Variables|Default|GetAcertos) 1))
      (if (== (Utilities|Array|LastIndex (Variables|Default|GetArrayDojogador)) (Utilities|Array|LastIndex (Variables|Default|GetArray)))
        ;[1 1 1] è a maior sequencia?
        (if (> _returnvalue (Variables|Default|GetMaiorSequencia))
          (Variables|Default|SetMaiorSequencia _returnvalue))
        (bind _outactors (Actor|GetAllActorsOfClass "/Game/Blueprints/BP_LuzCoringa.BP_LuzCoringa_C"))
        (for _array_element _outactors
          (Default|PiscarVerde _array_element))
        (Audio|PlaySound2D "/Game/Assets/Sons/CompletandoFase.CompletandoFase" 1.0 1.0 0.0 0 0)
        (Rendering|Material|SetMaterial (Variables|Default|GetVerde1) 0 "/Game/Materiais/Lazer_Verde.Lazer_Verde")
        (Rendering|Material|SetMaterial (Variables|Default|GetAmarelo4) 0 "/Game/Materiais/Lazer_Verde.Lazer_Verde")
        (Rendering|Material|SetMaterial (Variables|Default|GetVermelho3) 0 "/Game/Materiais/Lazer_Verde.Lazer_Verde")
        (Rendering|Material|SetMaterial (Variables|Default|GetAzul2) 0 "/Game/Materiais/Lazer_Verde.Lazer_Verde")
        (Utilities|Array|Clear (Variables|Default|GetArrayDojogador))
        (Utilities|FlowControl|Delay 0.5)
        (CallFunction|Apagar)
        (CallFunction|GerarSequencia)
        (CallFunction|IniciarSequencia)
        (else
          (Utilities|FlowControl|Delay 0.5)
          (CallFunction|Apagar)))
      (else
        ;[1 1 1] Erro
        (bind _outactors_2 (Actor|GetAllActorsOfClass "/Game/Blueprints/BP_LuzCoringa.BP_LuzCoringa_C"))
        (for _array_element_2 _outactors_2
          (Default|PiscarVermelho _array_element_2))
        (Audio|PlaySound2D "/Game/Assets/Sons/Wrong.Wrong" 1.0 1.0 0.0 0 0)
        (Rendering|Material|SetMaterial (Variables|Default|GetVerde1) 0 "/Game/Materiais/Lazer_Vermelho.Lazer_Vermelho")
        (Rendering|Material|SetMaterial (Variables|Default|GetAmarelo4) 0 "/Game/Materiais/Lazer_Vermelho.Lazer_Vermelho")
        (Rendering|Material|SetMaterial (Variables|Default|GetVermelho3) 0 "/Game/Materiais/Lazer_Vermelho.Lazer_Vermelho")
        (Rendering|Material|SetMaterial (Variables|Default|GetAzul2) 0 "/Game/Materiais/Lazer_Vermelho.Lazer_Vermelho")
        (Variables|Default|SetTentativasRestantes (- (Variables|Default|GetTentativasRestantes) 1))
        (Default|DiminuirContagem _referenciavidas)
        (UserInterface|SetWidget (Variables|Default|GetVidas) _referenciavidas)
        (if (== (Variables|Default|GetTentativasRestantes) 0)
          (bind _asgi_jogo (Utilities|Casting|CastToGI_Jogo (Game|GetGameInstance)))
          (Default|RegistrarFase2 _asgi_jogo (Variables|Default|GetAcertos) (Math|Float|Truncate (- (Utilities|Time|GetGameTimeinSeconds) (Variables|Default|GetTempoInicial))) (Variables|Default|GetMaiorSequencia))
          (bind _returnvalue_3 (UserInterface|CreateWidget "/Game/Widgets/FimFase2.FimFase2_C"))
          (UserInterface|Viewport|AddtoViewport _returnvalue_3 0)
          (else
            (Utilities|FlowControl|Delay 1.0)
            (CallFunction|Apagar)
            (Utilities|Array|Clear (Variables|Default|GetArrayDojogador))
            (Utilities|Array|Clear (Variables|Default|GetArray))
            (CallFunction|GerarSequencia)
            (CallFunction|IniciarSequencia)))))))

(event OnComponentHit(Azul2)
  (params (HitComponent :type Primitive%20Component%20Object%20Reference) (OtherActor :type Actor%20Object%20Reference) (OtherComp :type Primitive%20Component%20Object%20Reference) (NormalImpulse :type Vector :default "0, 0, 0") (Hit :type Hit%20Result%20Structure%20%28by%20ref%29))
  (bind _arraydojogador (Variables|Default|GetArrayDojogador))
  (bind _arraydojogador_2 (Variables|Default|GetArrayDojogador))
  (bind _referenciavidas (Variables|Default|GetReferenciaVidas))
  (bind _returnvalue (Utilities|Array|Length _arraydojogador))
  (bind _returnvalue_2 (Utilities|Array|LastIndex _arraydojogador_2))
  (if (not (Variables|Default|GetDesativarTiros))
    (Rendering|Material|SetMaterial (Variables|Default|GetAzul2) 0 "/Game/Materiais/Lazer_Azul.Lazer_Azul")
    (Audio|PlaySound2D "/Game/Assets/Sons/2.2" 1.0 1.0 0.0 0 0)
    (Utilities|Array|Add (Variables|Default|GetArrayDojogador) 2)
    (Utilities|FlowControl|Delay 0.2)
    (CallFunction|Apagar)
    (if (== (Utilities|Array|Get(acopy) (Variables|Default|GetArray) _returnvalue_2) (Utilities|Array|Get(acopy) (Variables|Default|GetArrayDojogador) _returnvalue_2))
      ;[1 1 1] Acertou/ é o ultimo acerto?
      (Variables|Default|SetAcertos (+ (Variables|Default|GetAcertos) 1))
      (if (== (Utilities|Array|LastIndex (Variables|Default|GetArrayDojogador)) (Utilities|Array|LastIndex (Variables|Default|GetArray)))
        ;[1 1 1] è a maior sequencia?
        (if (> _returnvalue (Variables|Default|GetMaiorSequencia))
          (Variables|Default|SetMaiorSequencia _returnvalue))
        (bind _outactors (Actor|GetAllActorsOfClass "/Game/Blueprints/BP_LuzCoringa.BP_LuzCoringa_C"))
        (for _array_element _outactors
          (Default|PiscarVerde _array_element))
        (Audio|PlaySound2D "/Game/Assets/Sons/CompletandoFase.CompletandoFase" 1.0 1.0 0.0 0 0)
        (Rendering|Material|SetMaterial (Variables|Default|GetVerde1) 0 "/Game/Materiais/Lazer_Verde.Lazer_Verde")
        (Rendering|Material|SetMaterial (Variables|Default|GetAmarelo4) 0 "/Game/Materiais/Lazer_Verde.Lazer_Verde")
        (Rendering|Material|SetMaterial (Variables|Default|GetVermelho3) 0 "/Game/Materiais/Lazer_Verde.Lazer_Verde")
        (Rendering|Material|SetMaterial (Variables|Default|GetAzul2) 0 "/Game/Materiais/Lazer_Verde.Lazer_Verde")
        (Utilities|Array|Clear (Variables|Default|GetArrayDojogador))
        (Utilities|FlowControl|Delay 0.5)
        (CallFunction|Apagar)
        (CallFunction|GerarSequencia)
        (CallFunction|IniciarSequencia)
        (else
          (Utilities|FlowControl|Delay 0.5)
          (CallFunction|Apagar)))
      (else
        ;[1 1 1] Erro
        (bind _outactors_2 (Actor|GetAllActorsOfClass "/Game/Blueprints/BP_LuzCoringa.BP_LuzCoringa_C"))
        (for _array_element_2 _outactors_2
          (Default|PiscarVermelho _array_element_2))
        (Audio|PlaySound2D "/Game/Assets/Sons/Wrong.Wrong" 1.0 1.0 0.0 0 0)
        (Rendering|Material|SetMaterial (Variables|Default|GetVerde1) 0 "/Game/Materiais/Lazer_Vermelho.Lazer_Vermelho")
        (Rendering|Material|SetMaterial (Variables|Default|GetAmarelo4) 0 "/Game/Materiais/Lazer_Vermelho.Lazer_Vermelho")
        (Rendering|Material|SetMaterial (Variables|Default|GetVermelho3) 0 "/Game/Materiais/Lazer_Vermelho.Lazer_Vermelho")
        (Rendering|Material|SetMaterial (Variables|Default|GetAzul2) 0 "/Game/Materiais/Lazer_Vermelho.Lazer_Vermelho")
        (Variables|Default|SetTentativasRestantes (- (Variables|Default|GetTentativasRestantes) 1))
        (Default|DiminuirContagem _referenciavidas)
        (UserInterface|SetWidget (Variables|Default|GetVidas) _referenciavidas)
        (if (== (Variables|Default|GetTentativasRestantes) 0)
          (bind _asgi_jogo (Utilities|Casting|CastToGI_Jogo (Game|GetGameInstance)))
          (Default|RegistrarFase2 _asgi_jogo (Variables|Default|GetAcertos) (Math|Float|Truncate (- (Utilities|Time|GetGameTimeinSeconds) (Variables|Default|GetTempoInicial))) (Variables|Default|GetMaiorSequencia))
          (bind _returnvalue_3 (UserInterface|CreateWidget "/Game/Widgets/FimFase2.FimFase2_C"))
          (UserInterface|Viewport|AddtoViewport _returnvalue_3 0)
          (else
            (Utilities|FlowControl|Delay 1.0)
            (CallFunction|Apagar)
            (Utilities|Array|Clear (Variables|Default|GetArrayDojogador))
            (Utilities|Array|Clear (Variables|Default|GetArray))
            (CallFunction|GerarSequencia)
            (CallFunction|IniciarSequencia)))))))

(event OnComponentHit(Vermelho3)
  (params (HitComponent :type Primitive%20Component%20Object%20Reference) (OtherActor :type Actor%20Object%20Reference) (OtherComp :type Primitive%20Component%20Object%20Reference) (NormalImpulse :type Vector :default "0, 0, 0") (Hit :type Hit%20Result%20Structure%20%28by%20ref%29))
  (bind _arraydojogador (Variables|Default|GetArrayDojogador))
  (bind _arraydojogador_2 (Variables|Default|GetArrayDojogador))
  (bind _referenciavidas (Variables|Default|GetReferenciaVidas))
  (bind _returnvalue (Utilities|Array|Length _arraydojogador))
  (bind _returnvalue_2 (Utilities|Array|LastIndex _arraydojogador_2))
  (if (not (Variables|Default|GetDesativarTiros))
    (Rendering|Material|SetMaterial (Variables|Default|GetVermelho3) 0 "/Game/Materiais/Lazer_Vermelho.Lazer_Vermelho")
    (Audio|PlaySound2D "/Game/Assets/Sons/3.3" 1.0 1.0 0.0 0 0)
    (Utilities|Array|Add (Variables|Default|GetArrayDojogador) 3)
    (Utilities|FlowControl|Delay 0.2)
    (CallFunction|Apagar)
    (if (== (Utilities|Array|Get(acopy) (Variables|Default|GetArray) _returnvalue_2) (Utilities|Array|Get(acopy) (Variables|Default|GetArrayDojogador) _returnvalue_2))
      ;[1 1 1] Acertou/ é o ultimo acerto?
      (Variables|Default|SetAcertos (+ (Variables|Default|GetAcertos) 1))
      (if (== (Utilities|Array|LastIndex (Variables|Default|GetArrayDojogador)) (Utilities|Array|LastIndex (Variables|Default|GetArray)))
        ;[1 1 1] è a maior sequencia?
        (if (> _returnvalue (Variables|Default|GetMaiorSequencia))
          (Variables|Default|SetMaiorSequencia _returnvalue))
        (bind _outactors (Actor|GetAllActorsOfClass "/Game/Blueprints/BP_LuzCoringa.BP_LuzCoringa_C"))
        (for _array_element _outactors
          (Default|PiscarVerde _array_element))
        (Audio|PlaySound2D "/Game/Assets/Sons/CompletandoFase.CompletandoFase" 1.0 1.0 0.0 0 0)
        (Rendering|Material|SetMaterial (Variables|Default|GetVerde1) 0 "/Game/Materiais/Lazer_Verde.Lazer_Verde")
        (Rendering|Material|SetMaterial (Variables|Default|GetAmarelo4) 0 "/Game/Materiais/Lazer_Verde.Lazer_Verde")
        (Rendering|Material|SetMaterial (Variables|Default|GetVermelho3) 0 "/Game/Materiais/Lazer_Verde.Lazer_Verde")
        (Rendering|Material|SetMaterial (Variables|Default|GetAzul2) 0 "/Game/Materiais/Lazer_Verde.Lazer_Verde")
        (Utilities|Array|Clear (Variables|Default|GetArrayDojogador))
        (Utilities|FlowControl|Delay 0.5)
        (CallFunction|Apagar)
        (CallFunction|GerarSequencia)
        (CallFunction|IniciarSequencia)
        (else
          (Utilities|FlowControl|Delay 0.5)
          (CallFunction|Apagar)))
      (else
        ;[1 1 1] Erro
        (bind _outactors_2 (Actor|GetAllActorsOfClass "/Game/Blueprints/BP_LuzCoringa.BP_LuzCoringa_C"))
        (for _array_element_2 _outactors_2
          (Default|PiscarVermelho _array_element_2))
        (Audio|PlaySound2D "/Game/Assets/Sons/Wrong.Wrong" 1.0 1.0 0.0 0 0)
        (Rendering|Material|SetMaterial (Variables|Default|GetVerde1) 0 "/Game/Materiais/Lazer_Vermelho.Lazer_Vermelho")
        (Rendering|Material|SetMaterial (Variables|Default|GetAmarelo4) 0 "/Game/Materiais/Lazer_Vermelho.Lazer_Vermelho")
        (Rendering|Material|SetMaterial (Variables|Default|GetVermelho3) 0 "/Game/Materiais/Lazer_Vermelho.Lazer_Vermelho")
        (Rendering|Material|SetMaterial (Variables|Default|GetAzul2) 0 "/Game/Materiais/Lazer_Vermelho.Lazer_Vermelho")
        (Variables|Default|SetTentativasRestantes (- (Variables|Default|GetTentativasRestantes) 1))
        (Default|DiminuirContagem _referenciavidas)
        (UserInterface|SetWidget (Variables|Default|GetVidas) _referenciavidas)
        (if (== (Variables|Default|GetTentativasRestantes) 0)
          (bind _asgi_jogo (Utilities|Casting|CastToGI_Jogo (Game|GetGameInstance)))
          (Default|RegistrarFase2 _asgi_jogo (Variables|Default|GetAcertos) (Math|Float|Truncate (- (Utilities|Time|GetGameTimeinSeconds) (Variables|Default|GetTempoInicial))) (Variables|Default|GetMaiorSequencia))
          (bind _returnvalue_3 (UserInterface|CreateWidget "/Game/Widgets/FimFase2.FimFase2_C"))
          (UserInterface|Viewport|AddtoViewport _returnvalue_3 0)
          (else
            (Utilities|FlowControl|Delay 1.0)
            (CallFunction|Apagar)
            (Utilities|Array|Clear (Variables|Default|GetArrayDojogador))
            (Utilities|Array|Clear (Variables|Default|GetArray))
            (CallFunction|GerarSequencia)
            (CallFunction|IniciarSequencia)))))))

(fn ConstructionScript)

(fn PiscarLuz
  (if (> (Variables|Default|GetContadorArray) (Utilities|Array|LastIndex (Variables|Default|GetArray)))
    (Class|KismetSystemLibrary|PauseTimer 0 "PiscarLuz")
    (Variables|Default|SetDesativarTiros false)
    (Utilities|Time|SetTimerbyFunctionName 0 "Apagar" 1.0)
    (else
      (switch int (Variables|Default|GetSeqAtual)
        (:0
          (Rendering|Material|SetMaterial (Variables|Default|GetVerde1) 0 "/Game/Materiais/Lazer_Verde.Lazer_Verde")
          (Audio|PlaySound2D "/Game/Assets/Sons/1.1" 1.0 1.0 0.0 0 0))
        (:1
          (Rendering|Material|SetMaterial (Variables|Default|GetAmarelo4) 0 "/Game/Materiais/Lazer_Amarelo.Lazer_Amarelo")
          (Audio|PlaySound2D "/Game/Assets/Sons/4.4" 1.0 1.0 0.0 0 0))
        (:2
          (Rendering|Material|SetMaterial (Variables|Default|GetAzul2) 0 "/Game/Materiais/Lazer_Azul.Lazer_Azul")
          (Audio|PlaySound2D "/Game/Assets/Sons/2.2" 1.0 1.0 0.0 0 0))
        (:3
          (Rendering|Material|SetMaterial (Variables|Default|GetVermelho3) 0 "/Game/Materiais/Lazer_Vermelho.Lazer_Vermelho")
          (Audio|PlaySound2D "/Game/Assets/Sons/3.3" 1.0 1.0 0.0 0 0)))
      (Audio|PlaySound2D 0 1.0 1.0 0.0 0 0)
      (Variables|Default|SetContadorArray (+ (Variables|Default|GetContadorArray) 1))
      (if (> (Variables|Default|GetContadorArray) (Utilities|Array|LastIndex (Variables|Default|GetArray)))
        _
        (else
          (Variables|Default|SetSeqAtual (Utilities|Array|Get(acopy) (Variables|Default|GetArray) (Variables|Default|GetContadorArray)))))
      (Utilities|Time|SetTimerbyFunctionName 0 "Apagar" 0.8))))

(fn GerarSequencia
  (Utilities|Array|Add (Variables|Default|GetArray) (Math|Random|RandomIntegerinRange 0 3)))

(fn IniciarSequencia
  (Variables|Default|SetDesativarTiros true)
  (Variables|Default|SetContadorArray 0)
  (Variables|Default|SetSeqAtual (Utilities|Array|Get(acopy) (Variables|Default|GetArray)))
  (Utilities|Array|Clear (Variables|Default|GetArrayDojogador))
  (Utilities|Time|SetTimerbyFunctionName 0 "PiscarLuz" (Variables|Default|GetTimerPiscar) true))

(fn Apagar
  (Rendering|Material|SetMaterial (Variables|Default|GetVerde1) 0 "/Game/Materiais/MT_LuzApagada.MT_LuzApagada")
  (Rendering|Material|SetMaterial (Variables|Default|GetAmarelo4) 0 "/Game/Materiais/MT_LuzApagada.MT_LuzApagada")
  (Rendering|Material|SetMaterial (Variables|Default|GetVermelho3) 0 "/Game/Materiais/MT_LuzApagada.MT_LuzApagada")
  (Rendering|Material|SetMaterial (Variables|Default|GetAzul2) 0 "/Game/Materiais/MT_LuzApagada.MT_LuzApagada"))

(fn ContarComecar
  (Variables|Default|SetDesativarTiros true)
  (bind _returnvalue (UserInterface|CreateWidget "/Game/Widgets/WB_Contagem.WB_Contagem_C"))
  (UserInterface|SetWidget (Variables|Default|GetContagem) _returnvalue)
  (Default|ComecarContagem _returnvalue)
  (EventDispatchers|BindEventtoComecaAgora5 _returnvalue (EventDispatchers|CreateEvent :!event Inicio)))

(fn Inicio
  (bind _returnvalue (Actor|GetActorOfClass "/Script/Engine.AmbientSound"))
  (Audio|Components|Audio|SetSound (Variables|/Script/Engine.AmbientSound|GetAudioComponent _returnvalue) "/Game/Assets/Sons/Musicas/BemLeve.BemLeve")
  (Class|AudioComponent|SetPaused (Variables|/Script/Engine.AmbientSound|GetAudioComponent _returnvalue) false)
  (Audio|Components|Audio|Play (Variables|/Script/Engine.AmbientSound|GetAudioComponent _returnvalue) 0.0)
  (Variables|Default|SetTempoInicial (Utilities|Time|GetGameTimeinSeconds))
  (bind _returnvalue_2 (UserInterface|CreateWidget "/Game/Widgets/WB_Vidas2fase.WB_Vidas2fase_C"))
  (bind _output_get (Variables|Default|SetReferenciaVidas _returnvalue_2))
  (UserInterface|SetWidget (Variables|Default|GetVidas) _output_get)
  (CallFunction|GerarSequencia)
  (CallFunction|IniciarSequencia))

(fn NewFunction)
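; BP_Gerador is a target generator that runs the timed first phase, keeping one target alive at a time.
; Começar starts the phase music and a looping timer on ChecarSpawn, which calls SpawnAlvo when no target lives.
; SpawnAlvo places a randomly scaled red, blue or green target on one face of the RegiaoSpawn box.
; At time-out, EncerrarGeracao destroys any remaining target and, only in that case, shows the FimFase1 widget with UI-only input.
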(event EventBeginPlay)

(fn ConstructionScript)

(fn ChecarSpawn
  (if (>= (Utilities|Time|GetGameTimeinSeconds) (Variables|Default|GetHoraFim))
    (Utilities|Time|ClearandInvalidateTimerbyHandle (Variables|Default|GetTimerChecagem))
    (Variables|Default|SetJanelaAtiva false)
    (CallFunction|EncerrarGeracao)
    (elif (Variables|Default|GetAlvoVivo)
      (Utilities|IsValid (Variables|Default|GetAlvoAtual)
        (:Is%20Not%20Valid
          (Variables|Default|SetAlvoVivo false)))
      (elif (and (not (Variables|Default|GetAlvoVivo)) (Variables|Default|GetJanelaAtiva))
        (CallFunction|SpawnAlvo)
        (else
          (Development|PrintString "deu ruim aq"))))))

(fn SpawnAlvo
  (bind _regiaospawn (Variables|Default|GetRegiaoSpawn))
  (bind _returnvalue (Transformation|GetWorldTransform _regiaospawn))
  (bind _returnvalue_2 (Components|Box|GetUnscaledBoxExtent _regiaospawn))
  (bind (_x _y _z) (Math|Vector|BreakVector _returnvalue_2))
  (bind _returnvalue_3 (* -1.0 _z))
  (bind _returnvalue_4 (* _y -1.0))
  (bind _returnvalue_5 (Math|Random|RandomFloatinRange _returnvalue_3 _z))
  (bind _returnvalue_6 (Math|Random|RandomFloatinRange _returnvalue_4 _y))
  (bind _returnvalue_7 (Math|Vector|MakeVector _x _returnvalue_6 _returnvalue_5))
  (bind _returnvalue_8 (Math|Transform|TransformLocation _returnvalue _returnvalue_7))
  (bind _returnvalue_9 (Math|Conversions|ToTransform(Vector) _returnvalue_8))
  (Audio|PlaySound2D "/Engine/EngineSounds/1kSineTonePing.1kSineTonePing" 1.0 1.0 0.0 0 0)
  (switch int (Math|Random|RandomIntegerinRange 0 2)
    (:0
      (bind _returnvalue_10 (Game|SpawnActorfromClass "/Game/Blueprints/BP_AlvoVermelho.BP_AlvoVermelho_C" _returnvalue_9 "AlwaysSpawn" "OverrideRootScale" 0 0))
      (Transformation|SetActorScale3D _returnvalue_10 (Math|Conversions|ToVector(Float) (Math|Random|RandomFloatinRange 0.9 2.0)))
      (bind _output_get (Variables|Default|SetAlvoAtual _returnvalue_10))
      (Utilities|IsValid _output_get
        (:Is%20Valid
          (Variables|Default|SetAlvoVivo true :!label _label))
        (:Is%20Not%20Valid
          (Development|PrintString "Falhou em spawnar" :!label _label_2))))
    (:1
      (bind _returnvalue_11 (Game|SpawnActorfromClass "/Game/Blueprints/BP_AlvoAzul.BP_AlvoAzul_C" _returnvalue_9 "Undefined" "OverrideRootScale" 0 0))
      (Transformation|SetActorScale3D _returnvalue_11 (Math|Conversions|ToVector(Float) (Math|Random|RandomFloatinRange 0.9 2.0)))
      (bind _output_get_2 (Variables|Default|SetAlvoAtual _returnvalue_11))
      (Utilities|IsValid _output_get_2
        (:Is%20Valid
          (goto _label))
        (:Is%20Not%20Valid
          (goto _label_2))))
    (:2
      (bind _returnvalue_12 (Game|SpawnActorfromClass "/Game/Blueprints/BP_AlvoVerde.BP_AlvoVerde_C" _returnvalue_9 "Undefined" "OverrideRootScale" 0 0))
      (Transformation|SetActorScale3D _returnvalue_12 (Math|Conversions|ToVector(Float) (Math|Random|RandomFloatinRange 0.9 2.0)))
      (bind _output_get_3 (Variables|Default|SetAlvoAtual _returnvalue_12))
      (Utilities|IsValid _output_get_3
        (:Is%20Valid
          (goto _label))
        (:Is%20Not%20Valid
          (goto _label_2))))))

(fn EncerrarGeracao
  (bind _returnvalue (Game|GetPlayerController 0))
  (bind _alvoatual (Variables|Default|GetAlvoAtual))
  (Variables|Default|SetJanelaAtiva true)
  (Utilities|IsValid _alvoatual
    (:Is%20Valid
      (Actor|DestroyActor _alvoatual)
      (bind _returnvalue_2 (UserInterface|CreateWidget "/Game/Widgets/FimFase1.FimFase1_C" _returnvalue))
      (UserInterface|Viewport|AddtoViewport _returnvalue_2 0)
      (Input|SetInputModeUIOnly _returnvalue 0 "DoNotLock" false)
      (Variables|/Script/Engine.PlayerController|SetbShowMouseCursor _returnvalue true))))

(fn Começar
  (bind _returnvalue (Actor|GetActorOfClass "/Script/Engine.AmbientSound"))
  (Audio|Components|Audio|SetSound (Variables|/Script/Engine.AmbientSound|GetAudioComponent _returnvalue) "/Game/Assets/Sons/Musicas/Fase_1_musica.Fase_1_musica")
  (Class|AudioComponent|SetPaused (Variables|/Script/Engine.AmbientSound|GetAudioComponent _returnvalue) false)
  (Audio|Components|Audio|Play (Variables|/Script/Engine.AmbientSound|GetAudioComponent _returnvalue) 0.5)
  (Variables|Default|SetJanelaAtiva true)
  (Variables|Default|SetAlvoVivo false)
  (Variables|Default|SetHoraFim (+ (Variables|Default|GetDucaraoJanelaSeg) (Utilities|Time|GetGameTimeinSeconds)))
  (bind _returnvalue_2 (Utilities|Time|SetTimerbyFunctionName 0 "ChecarSpawn" (Variables|Default|GetIntervaloChegagemSeg) true))
  (Variables|Default|SetTimerChecagem _returnvalue_2))
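; BP_AlvosIniciais spawns the initial set of red, blue and green target actors when play begins.
; BeginPlay creates them in sequence at hardcoded positions, spaced in a row along X at a shared Y and height, and stores each reference in its own variable.
; Only the red target forces AlwaysSpawn collision handling; the others leave it undefined.
; Tick, overlap and the construction script do nothing.
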(event EventBeginPlay
  (bind _returnvalue (Game|SpawnActorfromClass "/Game/Blueprints/BP_AlvoVermelho.BP_AlvoVermelho_C" (Math|Conversions|ToTransform(Vector) (Math|Vector|MakeVector 2.15e+03 45.0 2.2e+03)) "AlwaysSpawn" "OverrideRootScale" 0 0))
  (Variables|Default|Setvermelho _returnvalue)
  (bind _returnvalue_2 (Game|SpawnActorfromClass "/Game/Blueprints/BP_AlvoAzul.BP_AlvoAzul_C" (Math|Conversions|ToTransform(Vector) (Math|Vector|MakeVector 4.15e+03 45.0 2.2e+03)) "Undefined" "OverrideRootScale" 0 0))
  (Variables|Default|SetAzul _returnvalue_2)
  (bind _returnvalue_3 (Game|SpawnActorfromClass "/Game/Blueprints/BP_AlvoVerde.BP_AlvoVerde_C" (Math|Conversions|ToTransform(Vector) (Math|Vector|MakeVector 3.15e+03 45.0 2.2e+03)) "Undefined" "OverrideRootScale" 0 0))
  (Variables|Default|Setverde _returnvalue_3))

(event Collision|EventActorBeginOverlap
  (params (OtherActor :type Actor%20Object%20Reference)))

(event EventTick
  (params (DeltaSeconds :type Float%20%28single-precision%29)))

(fn ConstructionScript)
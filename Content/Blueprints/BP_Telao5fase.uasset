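; Big-screen quiz for phase 5, where hitting one of four components answers a multiple-choice logic question, mostly number sequences.
; Inicializar starts a countdown widget and fills a six-question bank.
; TrocarQuestão starts music and timer on first run, then shows a random question, recursively re-rolling answered ones.
; VerificarAcerto scores each hit with sound, and after three answers records results and time in GI_Jogo and shows FimFase5.
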(event OnComponentHit(1)
  (params (HitComponent :type Primitive%20Component%20Object%20Reference) (OtherActor :type Actor%20Object%20Reference) (OtherComp :type Primitive%20Component%20Object%20Reference) (NormalImpulse :type Vector :default "0, 0, 0") (Hit :type Hit%20Result%20Structure%20%28by%20ref%29))
  (Variables|Default|SetEscolha 1)
  (CallFunction|VerificarAcerto))

(event OnComponentHit(2)
  (params (HitComponent :type Primitive%20Component%20Object%20Reference) (OtherActor :type Actor%20Object%20Reference) (OtherComp :type Primitive%20Component%20Object%20Reference) (NormalImpulse :type Vector :default "0, 0, 0") (Hit :type Hit%20Result%20Structure%20%28by%20ref%29))
  (Variables|Default|SetEscolha 2)
  (CallFunction|VerificarAcerto))

(event OnComponentHit(3)
  (params (HitComponent :type Primitive%20Component%20Object%20Reference) (OtherActor :type Actor%20Object%20Reference) (OtherComp :type Primitive%20Component%20Object%20Reference) (NormalImpulse :type Vector :default "0, 0, 0") (Hit :type Hit%20Result%20Structure%20%28by%20ref%29))
  (Variables|Default|SetEscolha 3)
  (CallFunction|VerificarAcerto))

(event OnComponentHit(4)
  (params (HitComponent :type Primitive%20Component%20Object%20Reference) (OtherActor :type Actor%20Object%20Reference) (OtherComp :type Primitive%20Component%20Object%20Reference) (NormalImpulse :type Vector :default "0, 0, 0") (Hit :type Hit%20Result%20Structure%20%28by%20ref%29))
  (Variables|Default|SetEscolha 4)
  (CallFunction|VerificarAcerto))

(event Custom|CustomEvent
  (Utilities|Casting|CastToGI_Jogo (Game|GetGameInstance)
    (:then
      (UserInterface|CreateWidget "/Game/Widgets/WB_QuestaoLogica.WB_QuestaoLogica_C"))
    (:CastFailed
      (Development|PrintString "deu ruioni"))))

(event Collision|EventActorBeginOverlap
  (params (OtherActor :type Actor%20Object%20Reference)))

(event EventTick
  (params (DeltaSeconds :type Float%20%28single-precision%29)))

(event EventBeginPlay
  (Rendering|SetVisibility (Variables|Default|GetTela) false false))

(fn ConstructionScript)

(fn Inicializar
  (bind _returnvalue (UserInterface|CreateWidget "/Game/Widgets/WB_Contagem.WB_Contagem_C"))
  (UserInterface|SetWidget (Variables|Default|GetContagem) _returnvalue)
  (Default|ComecarContagem _returnvalue)
  (EventDispatchers|BindEventtoComecaAgora5 _returnvalue (EventDispatchers|CreateEvent :!event TrocarQuestão))
  (bind _output_get (Variables|Default|SetQuestao ""))
  (bind _structout (Utilities|Struct|SetmembersinES_Questao _output_get "Complete a sequência: 0, 1, 4, 9, 16, 25, 36, ____?" "45" "47" "49" "51" 3))
  (Utilities|Array|Add (Variables|Default|GetQuestoes) _structout)
  (bind _output_get_2 (Variables|Default|SetQuestao ""))
  (bind _structout_2 (Utilities|Struct|SetmembersinES_Questao _output_get_2 "Complete a sequência: 4, 16, 36, 64, ____?" "74" "75" "86" "100" 4))
  (Utilities|Array|Add (Variables|Default|GetQuestoes) _structout_2)
  (bind _output_get_3 (Variables|Default|SetQuestao ""))
  (bind _structout_3 (Utilities|Struct|SetmembersinES_Questao _output_get_3 "Complete a sequência: 1, 1, 2, 3, 5, 8, ____?" "10" "12" "13" "14" 3))
  (Utilities|Array|Add (Variables|Default|GetQuestoes) _structout_3)
  (bind _output_get_4 (Variables|Default|SetQuestao ""))
  (bind _structout_4 (Utilities|Struct|SetmembersinES_Questao _output_get_4 "Complete a sequência: 2, 10, 12, 16, 17, 18, 19, ____?" "200" "21" "22" "23" 1))
  (Utilities|Array|Add (Variables|Default|GetQuestoes) _structout_4)
  (bind _output_get_5 (Variables|Default|SetQuestao ""))
  (bind _structout_5 (Utilities|Struct|SetmembersinES_Questao _output_get_5 "Complete a sequência: 5, 11, 18, 26, 35, ____?" "43" "44" "45" "46" 3))
  (Utilities|Array|Add (Variables|Default|GetQuestoes) _structout_5)
  (bind _output_get_6 (Variables|Default|SetQuestao ""))
  (bind _structout_6 (Utilities|Struct|SetmembersinES_Questao _output_get_6 "Qual é o inverso de 0,2 ?" "2,0" "-0,2" "-2" "5" 4))
  (Utilities|Array|Add (Variables|Default|GetQuestoes) _structout_6))

(fn TrocarQuestão
  (if (Variables|Default|Getprimeiravez)
    (Rendering|SetVisibility (Variables|Default|GetTela) true true)
    (bind _returnvalue (Actor|GetActorOfClass "/Script/Engine.AmbientSound"))
    (Audio|Components|Audio|SetSound (Variables|/Script/Engine.AmbientSound|GetAudioComponent _returnvalue) "/Game/Assets/Sons/Musicas/Hora_de_pensar.Hora_de_pensar")
    (Class|AudioComponent|SetPaused (Variables|/Script/Engine.AmbientSound|GetAudioComponent _returnvalue) false)
    (Audio|Components|Audio|Play (Variables|/Script/Engine.AmbientSound|GetAudioComponent _returnvalue) 0.0)
    (Variables|Default|SetTempoInicio (Utilities|Time|GetGameTimeinSeconds))
    (Variables|Default|Setprimeiravez false))
  (bind _output_get (Variables|Default|Setindice (Math|Random|RandomIntegerinRange 0 5)))
  (if (== (Variables|Default|GetJarespondeu1) _output_get)
    (Development|PrintString "ja tem cumpade" :!label _label)
    (CallFunction|TrocarQuestão)
    (elif (== (Variables|Default|Getjarespondeu2) _output_get)
      (goto _label)
      (else
        (Variables|Default|Setquestãoatual (Utilities|Array|Get(acopy) (Variables|Default|GetQuestoes) (Variables|Default|Getindice)))
        (Default|SetarPergunta (Variables|Default|GetReferencia%20Tela) (.Pergunta (Utilities|Struct|BreakES_Questao (Utilities|Array|Get(acopy) (Variables|Default|GetQuestoes) (Variables|Default|Getindice)))) (.Alt1 (Utilities|Struct|BreakES_Questao (Utilities|Array|Get(acopy) (Variables|Default|GetQuestoes) (Variables|Default|Getindice)))) (.Alt2 (Utilities|Struct|BreakES_Questao (Utilities|Array|Get(acopy) (Variables|Default|GetQuestoes) (Variables|Default|Getindice)))) (.Alt3 (Utilities|Struct|BreakES_Questao (Utilities|Array|Get(acopy) (Variables|Default|GetQuestoes) (Variables|Default|Getindice)))) (.Alt4 (Utilities|Struct|BreakES_Questao (Utilities|Array|Get(acopy) (Variables|Default|GetQuestoes) (Variables|Default|Getindice)))) (.Correta (Utilities|Struct|BreakES_Questao (Utilities|Array|Get(acopy) (Variables|Default|GetQuestoes) (Variables|Default|Getindice)))))
        (UserInterface|SetWidget (Variables|Default|GetTela) (Variables|Default|GetReferencia%20Tela))))))

(fn VerificarAcerto
  (bind _indice (Variables|Default|Getindice))
  (if (== (Variables|Default|GetJarespondeu1) 100)
    (Variables|Default|SetJarespondeu1 _indice)
    (elif (== (Variables|Default|Getjarespondeu2) 100)
      (Variables|Default|Setjarespondeu2 _indice)))
  (if (== (.Correta (Utilities|Struct|BreakES_Questao (Variables|Default|Getquestãoatual))) (Variables|Default|GetEscolha))
    (Audio|PlaySound2D "/Game/Assets/Sons/AcertandoAlvo.AcertandoAlvo" 1.0 1.0 0.0 0 0)
    (Variables|Default|SetEscolha 0)
    (bind _output_get (Variables|Default|SetCertas (+ (Variables|Default|GetCertas) 1)))
    (else
      (Audio|PlaySound2D "/Game/Assets/Sons/Wrong.Wrong" 1.0 1.0 0.0 0 0)
      (Variables|Default|SetEscolha 0)
      (bind _output_get_2 (Variables|Default|SetErradas (+ (Variables|Default|GetErradas) 1)))))
  (if (> (+ _output_get _output_get_2) 2)
    (bind _asgi_jogo (Utilities|Casting|CastToGI_Jogo (Game|GetGameInstance)))
    (Default|RegistrarFase5 _asgi_jogo (Variables|Default|GetErradas) (Variables|Default|GetCertas) (Math|Float|Truncate (- (Utilities|Time|GetGameTimeinSeconds) (Variables|Default|GetTempoInicio))))
    (bind _returnvalue (UserInterface|CreateWidget "/Game/Widgets/FimFase5.FimFase5_C"))
    (UserInterface|Viewport|AddtoViewport _returnvalue 0)
    (else
      (CallFunction|TrocarQuestão))))
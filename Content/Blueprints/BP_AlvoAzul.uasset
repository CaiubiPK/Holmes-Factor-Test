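; Blue target actor that scores whether it is struck by a blue laser or by something else.
; A BP_LazerAzul hit plays a sound at the impact point, destroys the target and registers a hit in GI_Jogo, calling Comecar when F1Acertos reaches three.
; Any other hit registers an error in the game instance and plays a 2D wrong sound.
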(event EventBeginPlay
  (|CallParentFunction) ; This node is disabled and will not be called.\nDrag off pins to build functionality.
)

(event Collision|EventActorBeginOverlap
  (params (OtherActor :type Actor%20Object%20Reference))
  (|CallParentFunction OtherActor) ; This node is disabled and will not be called.\nDrag off pins to build functionality.
)

(event EventTick
  (params (DeltaSeconds :type Float%20%28single-precision%29))
  (|CallParentFunction DeltaSeconds) ; This node is disabled and will not be called.\nDrag off pins to build functionality.
)

(event Collision|EventHit
  (params (MyComp :type Primitive%20Component%20Object%20Reference) (Other :type Actor%20Object%20Reference) (OtherComp :type Primitive%20Component%20Object%20Reference) (bSelfMoved :type Boolean) (HitLocation :type Vector :default "0, 0, 0") (HitNormal :type Vector :default "0, 0, 0") (NormalImpulse :type Vector :default "0, 0, 0") (Hit :type Hit%20Result%20Structure%20%28by%20ref%29))
  (Utilities|Casting|CastToBP_LazerAzul Other
    (:then
      (Audio|PlaySoundatLocation "/Game/Assets/Sons/AcertandoAlvo.AcertandoAlvo" HitLocation "0, 0, 0" 1.0 1.0 0.0 0 0 0 0)
      (Actor|DestroyActor)
      (bind _asgi_jogo (Utilities|Casting|CastToGI_Jogo (Game|GetGameInstance))
        (:then
          (Default|RegistrarAcerto _asgi_jogo)
          (if (== (Variables|/Game/Blueprints/GI_Jogo.GI_Jogo_C|GetF1Acertos _asgi_jogo) 3)
            (Default|CallComecar)))
        (:CastFailed
          (Development|PrintString "Cast falou "))))
    (:CastFailed
      (bind _asgi_jogo_2 (Utilities|Casting|CastToGI_Jogo (Game|GetGameInstance))
        (:then
          (Default|RegistrarErro _asgi_jogo_2)
          (Audio|PlaySound2D "/Game/Assets/Sons/Wrong.Wrong" 1.0 1.0 0.0 0 0))
        (:CastFailed
          (Development|PrintText "deu ruim"))))))

(fn ConstructionScript
  (|CallParentFunction))
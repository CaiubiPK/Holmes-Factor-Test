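; BP_telao3D is an in-world screen actor that shows the countdown when a game round begins.
; On BeginPlay it binds to the Comecar dispatcher of the green, red and blue target actors.
; When that fires, it resets GI_Jogo data, puts a new WB_Contagem in its WidgetContagem component and starts the count.
; An older delay and timer countdown remains disconnected, and AtualizarContagem and FinalizarContagem are empty.
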(event Custom|CustomEvent
  (bind _asgi_jogo (Utilities|Casting|CastToGI_Jogo (Game|GetGameInstance)))
  (Default|ZerarDados _asgi_jogo)
  (bind _returnvalue (UserInterface|CreateWidget "/Game/Widgets/WB_Contagem.WB_Contagem_C"))
  (bind _output_get (Variables|Default|SetReferenvia _returnvalue))
  (UserInterface|SetWidget (Variables|Default|GetWidgetContagem) _output_get)
  (Default|ComecarContagem _output_get))

(event EventBeginPlay
  (bind _outactors (Actor|GetAllActorsOfClass "/Game/Blueprints/BP_AlvoVerde.BP_AlvoVerde_C"))
  (bind _outactors_2 (Actor|GetAllActorsOfClass "/Game/Blueprints/BP_AlvoVermelho.BP_AlvoVermelho_C"))
  (bind _outactors_3 (Actor|GetAllActorsOfClass "/Game/Blueprints/BP_AlvoAzul.BP_AlvoAzul_C"))
  (EventDispatchers|BindEventtoComecar _outactors (delegate Custom|CustomEvent))
  (EventDispatchers|BindEventtoComecar _outactors_2 (delegate Custom|CustomEvent))
  (EventDispatchers|BindEventtoComecar _outactors_3 (delegate Custom|CustomEvent)))

(event Collision|EventActorBeginOverlap
  (params (OtherActor :type Actor%20Object%20Reference)))

(event EventTick
  (params (DeltaSeconds :type Float%20%28single-precision%29)))

(fn ConstructionScript)

(fn AtualizarContagem)

(fn FinalizarContagem)
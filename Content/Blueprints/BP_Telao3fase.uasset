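; BP_Telao3fase is the phase 3 quiz screen, posing three logic questions from a hardcoded pool of eight in Portuguese.
; Inicializar starts a countdown widget and fills the pool; TrocarQuestão displays random questions, recursively rerolling ones already answered.
; Hits on four components choose answers; VerificarAcerto plays sounds, flashes BP_LuzCoringa lights and tallies results.
; After three answers it records score and time in GI_Jogo and shows FimFase3.
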(event OnComponentHit(1)
  (params (HitComponent :type Primitive%20Component%20Object%20Reference) (OtherActor :type Actor%20Object%20Reference) (OtherComp :type Primitive%20Component%20Object%20Reference) (NormalImpulse :type Vector :default "0, 0, 0") (Hit :type Hit%20Result%20Structure%20%28by%20ref%29))
  (Variables|Default|SetEscolha 1)
  (CallFunction|VerificarAcerto))

(event OnComponentHit(2)
  (params (HitComponent :type Primitive%20Component%20Object%20Reference) (OtherActor :type Actor%20Object%20Reference) (OtherComp :type Primitive%20Component%20Object%20Reference) (NormalImpulse :type Vector :default "0, 0, 0") (Hit :type Hit%20Result%20Structure%20%28by%20ref%29))
  (Variables|Default|SetEscolha 2)
  (CallFunction|VerificarAcerto))

(event OnComponentHit(3)
  (params (HitComponent :type Primitive%20Component%20Object%20Reference) (OtherActor :type Actor%20Object%20Reference) (OtherComp :type Primitive%20Component%20Object%20Reference) (NormalImpulse :type Vector :default "0, 0, 0") (Hit :type Hit%20Result%20Structure%20%28by%20ref%29))
  (Variables|Default|SetEscolha 3)
  (CallFunction|VerificarAcerto))

(event OnComponentHit(4)
  (params (HitComponent :type Primitive%20Component%20Object%20Reference) (OtherActor :type Actor%20Object%20Reference) (OtherComp :type Primitive%20Component%20Object%20Reference) (NormalImpulse :type Vector :default "0, 0, 0") (Hit :type Hit%20Result%20Structure%20%28by%20ref%29))
  (Variables|Default|SetEscolha 4)
  (CallFunction|VerificarAcerto))

(event EventBeginPlay
  (Rendering|SetVisibility (Variables|Default|GetTela) false false))

(fn ConstructionScript)

(fn Inicializar
  (bind _returnvalue (UserInterface|CreateWidget "/Game/Widgets/WB_Contagem.WB_Contagem_C"))
  (UserInterface|SetWidget (Variables|Default|GetContagem) _returnvalue)
  (Default|ComecarContagem _returnvalue)
  (EventDispatchers|BindEventtoComecaAgora5 _returnvalue (EventDispatchers|CreateEvent :!event TrocarQuestão))
  (bind _output_get (Variables|Default|SetQuestao ""))
  (bind _structout (Utilities|Struct|SetmembersinES_Questao _output_get "Em uma corrida com cinco participantes (Heitor, Carla, Marta, Jorge e Raul), temos as seguintes informações: 
 
- Marta não foi a última 
- Carla chegou logo antes de Jorge 
- Heitor chegou entre Carla e Raul. 
 
Quem foi o último colocado?" "Carla" "Heitor" "Jorge" "Raul " 4))
  (Utilities|Array|Add (Variables|Default|GetQuestoes) _structout)
  (bind _output_get_2 (Variables|Default|SetQuestao ""))
  (bind _structout_2 (Utilities|Struct|SetmembersinES_Questao _output_get_2 "Um número de três dígitos é igual à soma de seus dígitos multiplicada por 37. 
 
Qual é esse número?" "111" "333" "777" " Todos acima" 4))
  (Utilities|Array|Add (Variables|Default|GetQuestoes) _structout_2)
  (bind _output_get_3 (Variables|Default|SetQuestao ""))
  (bind _structout_3 (Utilities|Struct|SetmembersinES_Questao _output_get_3 "Em uma sala há 5 pessoas. Cada uma cumprimenta todas as outras exatamente uma vez. 
 
Quantos apertos de mão acontecem ao todo?" "8" "10" "15" "20" 2))
  (Utilities|Array|Add (Variables|Default|GetQuestoes) _structout_3)
  (bind _output_get_4 (Variables|Default|SetQuestao ""))
  (bind _structout_4 (Utilities|Struct|SetmembersinES_Questao _output_get_4 "Segundo o tratado internacional entre os países da América do Sul, se um avião cair exatamente entre a fronteira do Brasil e a Argentina,  
 
Onde devem ser enterrados os sobreviventes?" "Brasil" "Argentina" "De acordo com a nacionalidade " "Nenhum" 4))
  (Utilities|Array|Add (Variables|Default|GetQuestoes) _structout_4)
  (bind _output_get_5 (Variables|Default|SetQuestao ""))
  (bind _structout_5 (Utilities|Struct|SetmembersinES_Questao _output_get_5 "Em uma fazenda, há galinhas e vacas, somando um total de 32 cabeças e 86 patas. 
 
Quantas galinhas e quantas vacas há na fazenda?" "21 galinhas e 11 vacas " "19 galinhas e 14 vacas" "15 galinhas e 16 vacas" "20 galinhas e 12 vacas" 1))
  (Utilities|Array|Add (Variables|Default|GetQuestoes) _structout_5)
  (bind _output_get_6 (Variables|Default|SetQuestao ""))
  (bind _structout_6 (Utilities|Struct|SetmembersinES_Questao _output_get_6 "Numa agência telefônica, 2 telefonistas atendem 24 clientes em 4 horas.  
 
Mantidas as proporções, 5 telefonistas atendem quantos clientes em 4 horas?" "58 clientes  " " 60 clientes" "56 clientes" "54 clientes" 2))
  (Utilities|Array|Add (Variables|Default|GetQuestoes) _structout_6)
  (bind _output_get_7 (Variables|Default|SetQuestao ""))
  (bind _structout_7 (Utilities|Struct|SetmembersinES_Questao _output_get_7 "Três irmãos, Ana, Bruno e Carla têm idades que somadas resultam em 51 anos. Carla é 4 anos mais velha que a caçula, e Bruno, é separado por 2 anos de suas irmãs. 
 
Quantos anos tem o irmão mais velho?" "21" "17" "15" "19" 4))
  (Utilities|Array|Add (Variables|Default|GetQuestoes) _structout_7)
  (bind _output_get_8 (Variables|Default|SetQuestao ""))
  (bind _structout_8 (Utilities|Struct|SetmembersinES_Questao _output_get_8 "Se X é 3 vezes maior que Y e a soma de ambos é 20, qual é o valor de Y?" "4" "5" "6" "Nenhum" 2))
  (Utilities|Array|Add (Variables|Default|GetQuestoes) _structout_8))

(fn TrocarQuestão
  (if (Variables|Default|Getprimeiravez)
    (Rendering|SetVisibility (Variables|Default|GetTela) true true)
    (bind _returnvalue (Actor|GetActorOfClass "/Script/Engine.AmbientSound"))
    (Audio|Components|Audio|SetSound (Variables|/Script/Engine.AmbientSound|GetAudioComponent _returnvalue) "/Game/Assets/Sons/Musicas/Hora_de_pensar_2.Hora_de_pensar_2")
    (Class|AudioComponent|SetPaused (Variables|/Script/Engine.AmbientSound|GetAudioComponent _returnvalue) false)
    (Audio|Components|Audio|Play (Variables|/Script/Engine.AmbientSound|GetAudioComponent _returnvalue) 0.0)
    (Variables|Default|SetTempoInicio (Utilities|Time|GetGameTimeinSeconds))
    (Variables|Default|Setprimeiravez false))
  (bind _output_get (Variables|Default|Setindice (Math|Random|RandomIntegerinRange 0 7)))
  (if (== (Variables|Default|GetJarespondeu1) _output_get)
    (Development|PrintString "ja tem cumpade" :!label _label)
    (CallFunction|TrocarQuestão)
    (elif (== (Variables|Default|Getjarespondeu2) _output_get)
      (goto _label)
      (else
        (Variables|Default|Setquestãoatual (Utilities|Array|Get(acopy) (Variables|Default|GetQuestoes) (Variables|Default|Getindice)))
        (Default|SetarPergunta (Variables|Default|GetReferencia%20Tela) (.Pergunta (Utilities|Struct|BreakES_Questao (Utilities|Array|Get(acopy) (Variables|Default|GetQuestoes) (Variables|Default|Getindice)))) (.Alt1 (Utilities|Struct|BreakES_Questao (Utilities|Array|Get(acopy) (Variables|Default|GetQuestoes) (Variables|Default|Getindice)))) (.Alt2 (Utilities|Struct|BreakES_Questao (Utilities|Array|Get(acopy) (Variables|Default|GetQuestoes) (Variables|Default|Getindice)))) (.Alt3 (Utilities|Struct|BreakES_Questao (Utilities|Array|Get(acopy) (Variables|Default|GetQuestoes) (Variables|Default|Getindice)))) (.Alt4 (Utilities|Struct|BreakES_Questao (Utilities|Array|Get(acopy) (Variables|Default|GetQuestoes) (Variables|Default|Getindice)))) (.Correta (Utilities|Struct|BreakES_Questao (Utilities|Array|Get(acopy) (Variables|Default|GetQuestoes) (Variables|Default|Getindice)))))
        (UserInterface|SetWidget (Variables|Default|GetTela) (Variables|Default|GetReferencia%20Tela))))))

(fn VerificarAcerto
  (bind _indice (Variables|Default|Getindice))
  (if (== (Variables|Default|GetJarespondeu1) 100)
    (Variables|Default|SetJarespondeu1 _indice)
    (elif (== (Variables|Default|Getjarespondeu2) 100)
      (Variables|Default|Setjarespondeu2 _indice)))
  (if (== (.Correta (Utilities|Struct|BreakES_Questao (Variables|Default|Getquestãoatual))) (Variables|Default|GetEscolha))
    (Audio|PlaySound2D "/Game/Assets/Sons/AcertandoAlvo.AcertandoAlvo" 1.0 1.0 0.0 0 0)
    (bind _outactors (Actor|GetAllActorsOfClass "/Game/Blueprints/BP_LuzCoringa.BP_LuzCoringa_C"))
    (for _array_element _outactors
      (Default|PiscarVerde _array_element))
    (Variables|Default|SetEscolha 0)
    (bind _output_get (Variables|Default|SetCertas (+ (Variables|Default|GetCertas) 1)))
    (else
      (Audio|PlaySound2D "/Game/Assets/Sons/Wrong.Wrong" 1.0 1.0 0.0 0 0)
      (bind _outactors_2 (Actor|GetAllActorsOfClass "/Game/Blueprints/BP_LuzCoringa.BP_LuzCoringa_C"))
      (for _array_element_2 _outactors_2
        (Default|PiscarVermelho _array_element_2))
      (Variables|Default|SetEscolha 0)
      (bind _output_get_2 (Variables|Default|SetErradas (+ (Variables|Default|GetErradas) 1)))))
  (if (> (+ _output_get _output_get_2) 2)
    (bind _asgi_jogo (Utilities|Casting|CastToGI_Jogo (Game|GetGameInstance)))
    (Default|RegistrarFase3 _asgi_jogo (Variables|Default|GetCertas) (Variables|Default|GetErradas) (Math|Float|Truncate (- (Utilities|Time|GetGameTimeinSeconds) (Variables|Default|GetTempoInicio))))
    (bind _returnvalue (UserInterface|CreateWidget "/Game/Widgets/FimFase3.FimFase3_C"))
    (UserInterface|Viewport|AddtoViewport _returnvalue 0)
    (else
      (CallFunction|TrocarQuestão))))
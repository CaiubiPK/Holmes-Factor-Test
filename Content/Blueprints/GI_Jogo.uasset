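; Game instance (by its GI_ name) that stores player statistics for the game's five phases.
; Phase 1 counts shots, hits, wrong-ammo errors and longest hit streak; hits and errors also flash every BP_LuzCoringa green or red.
; Phases 2 to 5 each store results passed in by the caller.
; RegistrarFase1 and ZerarDados only reset Phase 1 counters; ZerarEstatisticasF1 also clears streaks, and NewFunction is empty.
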(fn RegistrarDisparo
  (Variables|Default|SetF1Disparos (+ (Variables|Default|GetF1Disparos) 1)))

(fn RegistrarAcerto
  (Variables|Default|SetF1Acertos (+ (Variables|Default|GetF1Acertos) 1))
  (Variables|Default|SetVariavelaxulixiarSequencia (+ (Variables|Default|GetVariavelaxulixiarSequencia) 1))
  (if (> (Variables|Default|GetVariavelaxulixiarSequencia) (Variables|Default|GetF1MaiorSequência))
    (Variables|Default|SetF1MaiorSequência (Variables|Default|GetVariavelaxulixiarSequencia)))
  (bind _outactors (Actor|GetAllActorsOfClass "/Game/Blueprints/BP_LuzCoringa.BP_LuzCoringa_C"))
  (for _array_element _outactors
    (Default|PiscarVerde _array_element)))

(fn ZerarEstatisticasF1
  (Variables|Default|SetF1Disparos 0)
  (Variables|Default|SetF1Acertos 0)
  (Variables|Default|SetF1MunicaoErrada 0)
  (Variables|Default|SetF1MaiorSequência 0)
  (Variables|Default|SetVariavelaxulixiarSequencia 0))

(fn RegistrarErro
  (Variables|Default|SetF1MunicaoErrada (+ (Variables|Default|GetF1MunicaoErrada) 1))
  (Variables|Default|SetVariavelaxulixiarSequencia 0)
  (bind _outactors (Actor|GetAllActorsOfClass "/Game/Blueprints/BP_LuzCoringa.BP_LuzCoringa_C"))
  (for _array_element _outactors
    (Default|PiscarVermelho _array_element)))

(fn RegistrarFase1
  (Variables|Default|SetF1Disparos 0)
  (Variables|Default|SetF1Acertos 0)
  (Variables|Default|SetF1MunicaoErrada 0))

(fn RegistrarFase2
  (params (Acertos :type Integer) (Tempo :type Integer) (MaiorSeq :type Integer))
  (Variables|Default|SetF2Acertos Acertos)
  (Variables|Default|SetF2MaiorSequencia MaiorSeq)
  (Variables|Default|SetF2Tempo Tempo))

(fn RegistrarFase3
  (params (Acertos :type Integer) (Erros :type Integer) (Tempo :type Integer))
  (Variables|Default|SetF3Acertos Acertos)
  (Variables|Default|SetF3Erros Erros)
  (Variables|Default|SetF3Tempo Tempo))

(fn RegistrarFase4
  (params (Tentativas :type Integer) (Tempo :type Integer) (TentativasIncorretas :type Integer))
  (Variables|Default|SetF4Tentativas Tentativas)
  (Variables|Default|SetF4Tempo Tempo)
  (Variables|Default|SetF4TentativasIncorretas TentativasIncorretas))

(fn RegistrarFase5
  (params (Erros :type Integer) (Acertos :type Integer) (Tempo :type Integer))
  (Variables|Default|SetF5Erros Erros)
  (Variables|Default|SetF5Acertos Acertos)
  (Variables|Default|SetF5Tempo Tempo))

(fn ZerarDados
  (Variables|Default|SetF1Acertos 0)
  (Variables|Default|SetF1Disparos 0)
  (Variables|Default|SetF1MunicaoErrada 0))

(fn NewFunction)